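; BoundaryForce_BP is a boundary volume that pushes physics bubbles inside its influence with a set force.
; Overlap events on the Boundary component add each PhysicsBubble_BP to an array on entry and remove it on exit.
; A looping timer started at BeginPlay periodically applies ForceAmount to every tracked bubble's collision as an acceleration change, so bubble mass is ignored.
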(event `self.ReceiveBeginPlay`
  ;[1 1 1] BeginPlay SetTimer for ApplyingForceToBubbles
  (`KismetSystemLibrary.K2_SetTimer` null "ApplyForceToBubbles" 0.5 true))

(event `ApplyForceToBubble`
  (params (Bubble :type "/Game/MyContent/LevelItems/Bubbles/PhysicsBubble_BP Object Reference"))
  ;[1 1 1] Apply Force to a Bubble
  (`PrimitiveComponent.AddForce` (`/Game/MyContent/LevelItems/Bubbles/PhysicsBubble_BP.BubbleCollision` Bubble) (`self.ForceAmount`) "None" true))

(event `ApplyForceToBubbles`
  ;[1 1 1] Apply Force to each Bubble in array
  (for _array_element (`self.Bubbles`)
    (`self.ApplyForceToBubble` _array_element)))

(event `self.Boundary.OnComponentBeginOverlap`
  (params (OverlappedComponent :type "PrimitiveComponent Object Reference") (OtherActor :type "Actor Object Reference") (OtherComp :type "PrimitiveComponent Object Reference") (OtherBodyIndex :type Integer) (bFromSweep :type Boolean) (SweepResult :type "HitResult Structure (by ref)"))
  ;[1 1 1] Add Bubble to Array when entering influence of Boundary
  (bind _asphysics_bubble_bp (cast `/Game/MyContent/LevelItems/Bubbles/PhysicsBubble_BP` OtherActor))
  (`KismetArrayLibrary.Array_Add` (`self.Bubbles`) _asphysics_bubble_bp))

(event `self.Boundary.OnComponentEndOverlap`
  (params (OverlappedComponent :type "PrimitiveComponent Object Reference") (OtherActor :type "Actor Object Reference") (OtherComp :type "PrimitiveComponent Object Reference") (OtherBodyIndex :type Integer))
  ;[1 1 1] Remove Bubble from Array when leaving influence of Boundary
  (bind _asphysics_bubble_bp (cast `/Game/MyContent/LevelItems/Bubbles/PhysicsBubble_BP` OtherActor))
  (`KismetArrayLibrary.Array_RemoveItem` (`self.Bubbles`) _asphysics_bubble_bp))

(fn `UserConstructionScript`)