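; Physics-driven bubble enemy that launches in a random direction, damages the player on contact, takes bullet damage and spawns puddles on the ground.
; Damping scales with mass, and a looping timer toggles merge readiness so touching bubbles can join.
; Splitting, merging and puddles go through BubbleSpawner_BP; shot-down bubbles award points and, except one size, drop random pickups.
; Freezing suspends physics and damage, while standing on a bubble galvanises it, briefly disabling gravity.
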(event `self.ReceiveBeginPlay`
  (bind _returnvalue (`PrimitiveComponent.GetMass` (`self.BubbleCollision`)))
  ;[1 1 1] BeginPlay - Set Direction Vector
  (bind _returnvalue_2 (`GameplayStatics.GetActorOfClass` "/Game/MyContent/Blueprints/BubbleSpawner_BP.BubbleSpawner_BP_C"))
  (set `self.BubbleSpawnerRef` _returnvalue_2)
  ;;[1 1 1] Create and Set the Force vector
  (bind _output_get (set `self.DirectionVector` (`KismetMathLibrary.MakeVector` (`KismetMathLibrary.RandomFloatInRange` -1.0 1.0) 0.0 (`KismetMathLibrary.RandomFloatInRange` 0.3 2.0))))
  ;;[1 1 1] Apply a force to the Bubble
  (`PrimitiveComponent.AddImpulse` (`self.BubbleCollision`) (* _output_get 1000.0) "None" false)
  ;;[1 1 1] Set Dampening respective to Size
  (`self.UpdateDampening` (* (`self.BubbleLinearDampeningFactor`) _returnvalue) (* (`self.BubbleAngularDampeningFactor`) _returnvalue))
  (`KismetSystemLibrary.K2_SetTimer` null "BubbleMergeActivation" 15.0 true 0.0 15.0)
  ;;[1 1 1] Calculate and Set Bubble Health
  (set `self.Health` (`self.MaxHealth`))
  ;;[1 1 1] Set the Special Item
  (`self.RandomSpecialItem`))

(event `self.ReceiveTick`
  (params (DeltaSeconds :type "Float (single-precision)"))
  ;[1 1 1] Am I dead, play death followed by dead animation
  (if (`self.IsFrozen`)
    (set `self.ElapsedTime` (+ DeltaSeconds (`self.ElapsedTime`)))
    (if (> (`self.ElapsedTime`) (`self.FrozenLifeSpan`))
      (`self.UnfreezeBubble`)
      (set `self.ElapsedTime` 0.0))
    (elif (`self.AmIDead`)
      (`/Engine/EditorBlueprintResources/StandardMacros.DoOnce` false :!label _label
        (:`Completed`
          (`PaperFlipbookComponent.SetFlipbook` (`self.PaperFlipbook`) "/Game/MyContent/LevelItems/Bubbles/FlipBooks/Bubble_Burst.Bubble_Burst")
          (`self.DisableInput` null)
          (`GameplayStatics.PlaySoundAtLocation` "/Game/MyContent/Audio/Bubblepop_0_6s_Cue.Bubblepop_0_6s_Cue" (`SceneComponent.K2_GetComponentLocation` (`self.BubbleCollision`)) (struct) 1.0 1.0 0.0 null null null)
          (`KismetSystemLibrary.Delay` 0.61)
          (cast `/Game/MyContent/Blueprints/BubbleGameInstance` (`GameplayStatics.GetGameInstance`))
          (`/Game/MyContent/Blueprints/BubbleSpawner_BP.DecrementBubbleAliveCount` (`self.BubbleSpawnerRef`))
          (`self.K2_DestroyActor`)
          (goto _label :!via `Reset`)))
      (else
        (if (`|EnumEquality` (`self.BubbleSize`) "NewEnumerator5")
          (set `self.IsReadyToJoin` false))
        ;;[1 1 1] Display Mass In Bubble
        (`TextRenderComponent.K2_SetText` (`self.TextRender`) (`KismetTextLibrary.Conv_DoubleToText` (`PrimitiveComponent.GetMass` (`self.BubbleCollision`)) "HalfToEven"))))))

(event `RandomSpecialItem`
  ;[1 1 1] Set the Special to Random Item
  (set `self.SpecialItem` (select `/Game/MyContent/Items/PickUps/BubblePickUpEnum` (cast `/Game/MyContent/Items/PickUps/BubblePickUpEnum` (`KismetMathLibrary.Conv_IntToByte` (`KismetMathLibrary.RandomIntegerInRange` 0 4))) :`NewEnumerator5` "NewEnumerator5" :`NewEnumerator0` "NewEnumerator0" :`NewEnumerator4` "NewEnumerator4" :`NewEnumerator3` "NewEnumerator3" :`NewEnumerator2` "NewEnumerator2" :!type "/Game/MyContent/Items/PickUps/BubblePickUpEnum Enum")))

(event `DropSpecialItem`
  (bind _returnvalue (`SceneComponent.K2_GetComponentLocation` (`self.BubbleCollision`)))
  ;[1 1 1] Drop Special Item
  (switch `/Game/MyContent/Items/PickUps/BubblePickUpEnum` (`self.SpecialItem`)
    (:`NewEnumerator0`
      (`|SpawnActorFromClass` "/Game/MyContent/Items/PickUps/AutoGun/AutoGunPickUp_BP.AutoGunPickUp_BP_C" (`KismetMathLibrary.MakeTransform` _returnvalue) "AlwaysSpawn" "OverrideRootScale" null null))
    (:`NewEnumerator4`
      (`|SpawnActorFromClass` "/Game/MyContent/Items/PickUps/Freeze/FreezePickup_BP.FreezePickup_BP_C" (`KismetMathLibrary.MakeTransform` _returnvalue) "AlwaysSpawn" "OverrideRootScale" self null))
    (:`NewEnumerator3`
      (`|SpawnActorFromClass` "/Game/MyContent/Items/PickUps/Health/HealthPickup_BP.HealthPickup_BP_C" (`KismetMathLibrary.MakeTransform` _returnvalue) "AlwaysSpawn" "OverrideRootScale" null null))
    (:`NewEnumerator2`
      (`|SpawnActorFromClass` "/Game/MyContent/Items/PickUps/WaterEvaporator/WaterEvaporatorPickup_BP.WaterEvaporatorPickup_BP_C" (`KismetMathLibrary.MakeTransform` _returnvalue) "AlwaysSpawn" "OverrideRootScale" null null))))

(event `FreezeBubble`
  ;[1 1 1] Freezing and Unfreezing
  ;;[1 1 1] Freeze the bubble
  (set `self.IsFrozen` true)
  (`PrimitiveComponent.SetPhysMaterialOverride` (`self.BubbleCollision`) null)
  (`PaperFlipbookComponent.SetFlipbook` (`self.PaperFlipbook`) "/Game/MyContent/LevelItems/Bubbles/FlipBooks/newFrozen_bubble_Flipbook.newFrozen_bubble_Flipbook")
  (`PrimitiveComponent.SetSimulatePhysics` (`self.BubbleCollision`) false))

(event `UnfreezeBubble`
  ;[1 1 1] Freezing and Unfreezing
  ;;[1 1 1] Unfreeze the Bubble and revert back to default settings
  (set `self.IsFrozen` false)
  (`PrimitiveComponent.SetPhysMaterialOverride` (`self.BubbleCollision`) "/Engine/EngineMaterials/PhysMat_Rubber.PhysMat_Rubber")
  (`PaperFlipbookComponent.SetFlipbook` (`self.PaperFlipbook`) "/Game/MyContent/LevelItems/Bubbles/FlipBooks/Bubble_Whole.Bubble_Whole")
  (`PrimitiveComponent.SetSimulatePhysics` (`self.BubbleCollision`) true))

(event `Galvanise`
  (bind _returnvalue (`PrimitiveComponent.GetMass` (`self.BubbleCollision`)))
  ;[1 1 1] Set the Gravity and the Galvanised Flipook, revert back after 5 seconds
  (`self.UpdateDampening` (`self.PlayerOnBubbleLinearDampening`) (`self.PlayerOnBubbleAngularDampening`))
  (`PrimitiveComponent.SetEnableGravity` (`self.BubbleCollision`) false)
  (`PaperFlipbookComponent.SetFlipbook` (`self.PaperFlipbook`) "/Game/MyContent/LevelItems/Bubbles/FlipBooks/Bubble_Galvanised.Bubble_Galvanised")
  (`KismetSystemLibrary.Delay` 5.0)
  (`PrimitiveComponent.SetEnableGravity` (`self.BubbleCollision`) true)
  (`PaperFlipbookComponent.SetFlipbook` (`self.PaperFlipbook`) "/Game/MyContent/LevelItems/Bubbles/FlipBooks/Bubble_Whole.Bubble_Whole")
  (`self.UpdateDampening` (* (`self.BubbleLinearDampeningFactor`) _returnvalue) (* (`self.BubbleAngularDampeningFactor`) _returnvalue)))

(event `BubbleMergeActivation`
  ;[1 1 1] Enable Bubble Merge on FlipFlop
  (`/Engine/EditorBlueprintResources/StandardMacros.FlipFlop`
    (:`A`
      (set `self.IsReadyToJoin` true))
    (:`B`
      (set `self.IsReadyToJoin` false))))

(event `JoinBubbles`
  (params (TouchingBubble :type "/Game/MyContent/LevelItems/Bubbles/PhysicsBubble_BP Object Reference"))
  ;[1 1 1] Join touching bubble with self and destroy touching bubble
  (if (and (`self.IsReadyToJoin`) (`/Game/MyContent/LevelItems/Bubbles/PhysicsBubble_BP.IsReadyToJoin` TouchingBubble))
    (`/Engine/EditorBlueprintResources/StandardMacros.DoOnce` false
      (:`Completed`
        (`/Game/MyContent/Blueprints/BubbleSpawner_BP.MergeBubbles` (`self.BubbleSpawnerRef`) self TouchingBubble (`SceneComponent.K2_GetComponentLocation` (`self.BubbleCollision`)))))))

(event `UpdateDampening`
  (params (LinearValue :type "Float (double-precision)") (AngularValue :type "Float (double-precision)"))
  (bind _bubblecollision (`self.BubbleCollision`))
  ;[1 1 1] Update the Linear and Angular Dampening of the Bubble
  (`PrimitiveComponent.SetLinearDamping` _bubblecollision LinearValue)
  (`PrimitiveComponent.SetAngularDamping` _bubblecollision AngularValue))

(event `self.SphereOfInfluence.OnComponentBeginOverlap`
  (params (OverlappedComponent :type "PrimitiveComponent Object Reference") (OtherActor :type "Actor Object Reference") (OtherComp :type "PrimitiveComponent Object Reference") (OtherBodyIndex :type Integer) (bFromSweep :type Boolean) (SweepResult :type "HitResult Structure (by ref)"))
  ;[1 1 1] Is Player within radius of oversight
  (cast `/Game/MyContent/Characters/BubbleCharacter/BubbleCharacter` OtherActor)
  (set `self.IsOverlapping` true))

(event `self.SphereOfInfluence.OnComponentEndOverlap`
  (params (OverlappedComponent :type "PrimitiveComponent Object Reference") (OtherActor :type "Actor Object Reference") (OtherComp :type "PrimitiveComponent Object Reference") (OtherBodyIndex :type Integer))
  ;[1 1 1] Is Player within radius of oversight
  (cast `/Game/MyContent/Characters/BubbleCharacter/BubbleCharacter` OtherActor)
  (set `self.IsOverlapping` false))

(event `self.BubbleCollision.OnComponentBeginOverlap`
  (params (OverlappedComponent :type "PrimitiveComponent Object Reference") (OtherActor :type "Actor Object Reference") (OtherComp :type "PrimitiveComponent Object Reference") (OtherBodyIndex :type Integer) (bFromSweep :type Boolean) (SweepResult :type "HitResult Structure (by ref)"))
  ;[1 1 1] Bubble touches another bubble, try to join them
  (bind _asphysics_bubble_bp (cast `/Game/MyContent/LevelItems/Bubbles/PhysicsBubble_BP` OtherActor)
    (:`then`
      (`self.JoinBubbles` _asphysics_bubble_bp))
    (:`CastFailed`
      ;[1 1 1] Bubble Hits Player
      (bind _asbubble_character (cast `/Game/MyContent/Characters/BubbleCharacter/BubbleCharacter` OtherActor)
        (:`then`
          (`/Game/MyContent/Characters/BubbleCharacter/BubbleCharacter.UpdateHealth` _asbubble_character -25.0)
          (set `self.AmIDead` true))
        (:`CastFailed`
          ;[1 1 1] Bubble Hits Ground
          (cast `/Game/MyContent/LevelItems/Floors/Actors/BubbleGround_BP` OtherActor
            (:`then`
              _)
            (:`CastFailed`
              (cast `/Game/MyContent/LevelItems/Floors/Actors/BaseGroundContinous_BP` OtherActor
                (:`then`
                  _)
                (:`CastFailed`
                  (cast `/Game/MyContent/LevelItems/Floors/Actors/BaseGroundLeft_BP` OtherActor
                    (:`then`
                      _)
                    (:`CastFailed`
                      (cast `/Game/MyContent/LevelItems/Floors/Actors/BaseGroundRight_BP` OtherActor)))))))
          (`self.BubbleHitGround`))))))

(event `PopSelf`
  ;[1 1 1] Destroy Self
  (`KismetSystemLibrary.Delay` 0.2)
  (set `self.AmIDead` true))

(event `self.BubbleCollision.OnComponentHit`
  (params (HitComponent :type "PrimitiveComponent Object Reference") (OtherActor :type "Actor Object Reference") (OtherComp :type "PrimitiveComponent Object Reference") (NormalImpulse :type "Vector Structure") (Hit :type "HitResult Structure (by ref)"))
  ;[1 1 1] Bubble Hit by Bubble, Player or Bullet
  ;;[1 1 1] Bubble shall take no damage whilst frozen
  (if (not (`self.IsFrozen`))
    ;;[1 1 1] Bubbles touch and shall Join
    (bind _asphysics_bubble_bp (cast `/Game/MyContent/LevelItems/Bubbles/PhysicsBubble_BP` OtherActor)
      (:`then`
        (`self.JoinBubbles` _asphysics_bubble_bp))
      (:`CastFailed`
        ;;[1 1 1] Bullet hits Bubble, reduce health
        (bind _asbullet_bp (cast `/Game/MyContent/Projectiles/Bullet_BP` OtherActor)
          (:`then`
            (`self.K2_DestroyActor` _asbullet_bp)
            (bind _output_get (set `self.Health` (- (`self.Health`) 100.0)))
            ;;[1 1 1] Check Health of Bubble
            (if (> _output_get 0.0)
              ;;[1 1 1] Bubble has health, and play bubble hit sound
              (`GameplayStatics.PlaySoundAtLocation` "/Game/GameSoundCollection/Cartoon/Cue/Cartoon_dung_exp_Cue.Cartoon_dung_exp_Cue" (`SceneComponent.K2_GetComponentLocation` (`self.BubbleCollision`)) (struct) 1.0 1.0 0.0 null null null)
              (else
                ;;[1 1 1] Bubble no health, Update player score, Pop Bubble
                (bind _asbubble_character (cast `/Game/MyContent/Characters/BubbleCharacter/BubbleCharacter` (`GameplayStatics.GetPlayerCharacter` 0)))
                (`/Engine/EditorBlueprintResources/StandardMacros.DoOnce` false
                  (:`Completed`
                    (`/Game/MyContent/Characters/BubbleCharacter/BubbleCharacter.UpdateScoreMsg` _asbubble_character (`self.PointValue`))
                    (if (`|EnumInequality` (`self.BubbleSize`) "NewEnumerator4")
                      (`/Game/MyContent/Blueprints/BubbleSpawner_BP.PopBubble` (`self.BubbleSpawnerRef`) (`self.BubbleSize`) (`SceneComponent.K2_GetComponentLocation` (`self.BubbleCollision`)))
                      ;;[1 1 1] Initiate Death Sequence
                      (set `self.AmIDead` true)
                      ;;[1 1 1] Drop the Special Item
                      (`self.DropSpecialItem`)
                      (else
                        (set `self.AmIDead` true))))))))
          (:`CastFailed`
            ;;[1 1 1] Player hits Bubble
            (bind _asbubble_character_2 (cast `/Game/MyContent/Characters/BubbleCharacter/BubbleCharacter` OtherActor))
            (bind _playerabovebubble (`self.Is Player Above`))
            (if _playerabovebubble
              ;;;[1 1 1] Player is standing on Bubble, Galvanise Bubble
              (`self.Galvanise`)
              (else
                ;;;[1 1 1] Player hits the bubble, reduce the health, set to death
                (`/Game/MyContent/Characters/BubbleCharacter/BubbleCharacter.UpdateHealth` _asbubble_character_2 -5.0)
                (set `self.AmIDead` true)))))))))

(fn `BubbleHitGround`
  (`/Game/MyContent/Blueprints/BubbleSpawner_BP.SpawnPuddle` (`self.BubbleSpawnerRef`) (`SceneComponent.K2_GetComponentLocation` (`self.BubbleCollision`)) (`self.BubbleSize`))
  (`/Engine/EditorBlueprintResources/StandardMacros.DoOnce` false
    (:`Completed`
      (set `self.AmIDead` true))))

(fn `Is Player Above`
  (returns (playerAboveBubble :type Boolean))
  (bind (_returnvalue_x _returnvalue_y _returnvalue_z) (`KismetMathLibrary.BreakVector` (`SceneComponent.K2_GetComponentLocation` (`self.BubbleCollision`))))
  ;[1 1 1] Check Player is above Bubble and Set PlayerOnBubble repesctively
  (bind _asbubble_character (cast `/Game/MyContent/Characters/BubbleCharacter/BubbleCharacter` (`GameplayStatics.GetPlayerCharacter` 0)))
  (bind (_returnvalue_x_2 _returnvalue_y_2 _returnvalue_z_2) (`KismetMathLibrary.BreakVector` (`SceneComponent.K2_GetComponentLocation` (`Character.CapsuleComponent` _asbubble_character))))
  (if (> _returnvalue_z_2 _returnvalue_z)
    (return true)
    (else
      (return false))))

(fn `UserConstructionScript`)