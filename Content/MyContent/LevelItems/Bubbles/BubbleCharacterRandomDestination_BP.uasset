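; Paper2D bubble enemy that wanders the X/Z plane and chases the player inside its SphereOfInfluence.
; A looping timer picks random destinations and another spawns markers there, while Tick steers toward the player or destination.
; Touching the player deals damage and pops the bubble; bullet hits reduce its Health and award points on a kill.
; Death plays a burst flipbook and sound, then destroys the actor.
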(event `HitByAttack`
  ;[1 1 1] Play Damage Animation
  (`PaperFlipbookComponent.SetFlipbook` (`self.Sprite`) "/Game/MyContent/LevelItems/Bubbles/FlipBooks/Bubble_Hurt.Bubble_Hurt"))

(event `self.ReceiveBeginPlay`
  ;[1 1 1] BeginPlay - Set Destination Timer
  (`self.SetDestination`)
  (`self.ShowDestinationMarker`)
  (`KismetSystemLibrary.K2_SetTimer` null "SetDestination" 5.0 true)
  (`KismetSystemLibrary.Delay` 0.2)
  (`KismetSystemLibrary.K2_SetTimer` null "ShowDestinationMarker" 3.0 true))

(event `UpdateAnimation`
  ;[1 1 1] Handle Animation
  (if (`NavMovementComponent.IsFalling` (`self.CharacterMovement`))
    (`PaperFlipbookComponent.SetFlipbook` (`self.Sprite`) "/Game/MyContent/LevelItems/Bubbles/FlipBooks/Bubble_Whole.Bubble_Whole")
    (else
      (`PaperFlipbookComponent.SetFlipbook` (`self.Sprite`) (select `bool` (> (`KismetMathLibrary.VSize` (`self.GetVelocity`)) 0.0) :`false` "/Game/MyContent/LevelItems/Bubbles/FlipBooks/Bubble_Whole.Bubble_Whole" :`true` "/Game/MyContent/LevelItems/Bubbles/FlipBooks/Bubble_Whole.Bubble_Whole" :!type "PaperFlipbook Object Reference")))))

(event `InputAxis|Move`
  (params (AxisValue :type "Float (single-precision)"))
  ;[1 1 1] Handle movement
  (if (> AxisValue 0.0)
    (set `self.bisMovingRight` true)
    (elif (< AxisValue 0.0)
      (set `self.bisMovingRight` false)))
  (`self.AddMovementInput` (1.0 0.0 0.0) AxisValue))

(event `self.ReceiveTick`
  (params (DeltaSeconds :type "Float (single-precision)"))
  (bind (_destination_x _destination_y _destination_z) (`KismetMathLibrary.BreakVector` (`self.Destination`)))
  (bind _destination_x_2 (`KismetMathLibrary.BreakVector` (`self.Destination`)))
  (bind _returnvalue_x (`KismetMathLibrary.BreakVector` (`SceneComponent.K2_GetComponentLocation` (`self.CapsuleComponent`))))
  (bind (_returnvalue_x_2 _returnvalue_y _returnvalue_z) (`KismetMathLibrary.BreakVector` (`SceneComponent.K2_GetComponentLocation` (`self.CapsuleComponent`))))
  (bind (_returnvalue_x_3 _returnvalue_y_2 _returnvalue_z_2) (`KismetMathLibrary.BreakVector` (`SceneComponent.K2_GetComponentLocation` (`self.CapsuleComponent`))))
  (bind _returnvalue_x_4 (`KismetMathLibrary.BreakVector` (`SceneComponent.K2_GetComponentLocation` (`self.CapsuleComponent`))))
  (bind _returnvalue (- _destination_z _returnvalue_z_2))
  (bind _returnvalue_2 (- _destination_x_2 _returnvalue_x_4))
  ;[1 1 1] Tick - Updates animation
  ;;[1 1 1] Am I dead, play death followed by dead animation
  (if (`self.AmIDead`)
    (`/Engine/EditorBlueprintResources/StandardMacros.DoOnce` false
      (:`Completed`
        (`PaperFlipbookComponent.SetFlipbook` (`self.Sprite`) "/Game/MyContent/LevelItems/Bubbles/FlipBooks/Bubble_Burst.Bubble_Burst")
        (`self.DisableInput` null)
        (`GameplayStatics.PlaySoundAtLocation` "/Game/MyContent/Audio/Bubblepop_0_6s_Cue.Bubblepop_0_6s_Cue" (`SceneComponent.K2_GetComponentLocation` (`self.CapsuleComponent`)) (struct) 1.0 1.0 0.0 null null null)
        (`KismetSystemLibrary.Delay` 0.6)
        (`self.K2_DestroyActor`)))
    (elif (`self.IsHit`)
      (`self.HitByAttack`)
      ;;[1 1 1] Update movement animation
      (`/Engine/EditorBlueprintResources/StandardMacros.CompareFloat` (.x (`MovementComponent.Velocity` (`self.GetMovementComponent`))) :!label _label
        (:`>`
          ;;[1 1 1] Correct Rotation for left and right sprite movement
          (`self.K2_SetActorRotation` (`KismetMathLibrary.MakeRotator` 0.0) :!label _label_2))
        (:`==`
          (if (`self.bisMovingRight`)
            (goto _label_2)
            (else
              (`self.K2_SetActorRotation` (`KismetMathLibrary.MakeRotator` 0.0 0.0 180.0) :!label _label_3))))
        (:`<`
          (goto _label_3)))
      ;;[1 1 1] Increase Stamina
      (set `self.Stamina` (+ (`self.Stamina`) 0.05))
      ;;[1 1 1] Am I dead?
      (if (<= (`self.Health`) 0.0)
        (set `self.AmIDead` true))
      (elif (`self.IsOverlapping`)
        (bind _asbubble_character (cast `/Game/MyContent/Characters/BubbleCharacter/BubbleCharacter` (`GameplayStatics.GetPlayerCharacter` 0)))
        (`|ExecutionSequence`
          (:`then_0`
            (bind _returnvalue_x_5 (`KismetMathLibrary.BreakVector` (`SceneComponent.K2_GetComponentLocation` (`Character.CapsuleComponent` _asbubble_character))))
            (bind _returnvalue_3 (- _returnvalue_x_5 _returnvalue_x))
            ;;[1 1 1] Move X Axis (Left/Righr)
            (if (>= _returnvalue_3 0.0)
              (set `self.bisMovingRight` true)
              (else
                (set `self.bisMovingRight` false)))
            (`self.AddMovementInput` (1.0 0.0 0.0) _returnvalue_3))
          (:`then_1`
            (bind (_returnvalue_x_6 _returnvalue_y_3 _returnvalue_z_3) (`KismetMathLibrary.BreakVector` (`SceneComponent.K2_GetComponentLocation` (`Character.CapsuleComponent` _asbubble_character))))
            (bind _returnvalue_4 (- _returnvalue_z_3 _returnvalue_z))
            ;;[1 1 1] Move Z Axis (Up/Down)
            (if (>= _returnvalue_4 0.0)
              (set `self.bIsMovingUp` true)
              (else
                (set `self.bIsMovingUp` false)))
            (`self.AddMovementInput` (0.0 0.0 1.0) _returnvalue_4)))
        (elif (not (`self.DestinationReached`))
          (`|ExecutionSequence`
            (:`then_0`
              ;;[1 1 1] Move X Axis (Left/Righr)
              (if (>= _returnvalue_2 0.0)
                (set `self.bisMovingRight` true)
                (else
                  (set `self.bisMovingRight` false)))
              (`self.AddMovementInput` (1.0 0.0 0.0) _returnvalue_2))
            (:`then_1`
              ;;[1 1 1] Move Z Axis (Up/Down)
              (if (>= _returnvalue 0.0)
                (set `self.bIsMovingUp` true)
                (else
                  (set `self.bIsMovingUp` false)))
              (`self.AddMovementInput` (0.0 0.0 1.0) _returnvalue)))
          (else
            (`self.UpdateAnimation`)
            (goto _label)))))))

(event `InputAxis MoveUp`
  (params (`Axis value` :type "Float (double-precision)"))
  ;[1 1 1] Handle movement
  (if (> `Axis value` 0.0)
    (set `self.bIsMovingUp` true)
    (elif (< `Axis value` 0.0)
      (set `self.bIsMovingUp` false)))
  (`self.AddMovementInput` (0.0 0.0 0.0) `Axis value`))

(event `self.SphereOfInfluence.OnComponentBeginOverlap`
  (params (OverlappedComponent :type "PrimitiveComponent Object Reference") (OtherActor :type "Actor Object Reference") (OtherComp :type "PrimitiveComponent Object Reference") (OtherBodyIndex :type Integer) (bFromSweep :type Boolean) (SweepResult :type "HitResult Structure (by ref)"))
  ;[1 1 1] Is Player within radius of oversight
  (cast `/Game/MyContent/Characters/BubbleCharacter/BubbleCharacter` OtherActor)
  (set `self.IsOverlapping` true))

(event `self.SphereOfInfluence.OnComponentEndOverlap`
  (params (OverlappedComponent :type "PrimitiveComponent Object Reference") (OtherActor :type "Actor Object Reference") (OtherComp :type "PrimitiveComponent Object Reference") (OtherBodyIndex :type Integer))
  ;[1 1 1] Is Player within radius of oversight
  (cast `/Game/MyContent/Characters/BubbleCharacter/BubbleCharacter` OtherActor)
  (set `self.IsOverlapping` false))

(event `self.BubbleCollision.OnComponentBeginOverlap`
  (params (OverlappedComponent :type "PrimitiveComponent Object Reference") (OtherActor :type "Actor Object Reference") (OtherComp :type "PrimitiveComponent Object Reference") (OtherBodyIndex :type Integer) (bFromSweep :type Boolean) (SweepResult :type "HitResult Structure (by ref)"))
  ;[1 1 1] Bubble Hits Player
  (bind _asbubble_character (cast `/Game/MyContent/Characters/BubbleCharacter/BubbleCharacter` OtherActor))
  (set `/Game/MyContent/Characters/BubbleCharacter/BubbleCharacter.Health` (- (`/Game/MyContent/Characters/BubbleCharacter/BubbleCharacter.Health` _asbubble_character) 25.0) _asbubble_character)
  (set `self.AmIDead` true))

(event `self.BubbleCollision.OnComponentHit`
  (params (HitComponent :type "PrimitiveComponent Object Reference") (OtherActor :type "Actor Object Reference") (OtherComp :type "PrimitiveComponent Object Reference") (NormalImpulse :type "Vector Structure") (Hit :type "HitResult Structure (by ref)"))
  ;[1 1 1] Bubble Hit by Bullets
  (cast `/Game/MyContent/Projectiles/Bullet_BP` OtherActor)
  (if (not (`self.AmIDead`))
    (bind _output_get (set `self.Health` (- (`self.Health`) 25.0)))
    (if (> _output_get 0.0)
      (`GameplayStatics.PlaySoundAtLocation` "/Game/GameSoundCollection/Cartoon/Cue/Cartoon_dung_exp_Cue.Cartoon_dung_exp_Cue" (`SceneComponent.K2_GetComponentLocation` (`self.CapsuleCollision`)) (struct) 1.0 1.0 0.0 null null null)
      (else
        (set `self.AmIDead` true)
        (bind _asbubble_character (cast `/Game/MyContent/Characters/BubbleCharacter/BubbleCharacter` (`GameplayStatics.GetPlayerCharacter` 0)))
        (`/Game/MyContent/Characters/BubbleCharacter/BubbleCharacter.ChangeScore` _asbubble_character (`self.PointValue`))))))

(fn `DestinationReached?`
  (set `self.DestinationReached` (== (`self.Destination`) (`SceneComponent.K2_GetComponentLocation` (`self.CapsuleComponent`)) :`ErrorTolerance` 250.0)))

(fn `SetDestination`
  (set `self.DestinationReached` false)
  (set `self.Destination` (`KismetMathLibrary.MakeVector` (`KismetMathLibrary.RandomFloatInRange` -3000.0 3000.0) 0.0 (`KismetMathLibrary.RandomFloatInRange` -3000.0 3000.0))))

(fn `ShowDestinationMarker`
  (`|SpawnActorFromClass` "/Game/MyContent/LevelItems/Bubbles/DestinationMarker/DestinationMarker_BP.DestinationMarker_BP_C" (`KismetMathLibrary.MakeTransform` (`self.Destination`)) "AlwaysSpawn" "OverrideRootScale" null null))

(fn `UserConstructionScript`)