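; Water puddle hazard that slowly sinks and damages the player's BubbleCharacter while standing in it.
; A looping timer nudges the root downward with sweep, and a text render shows PuddleSize every tick.
; Sprite overlaps set an in-water flag, which Tick checks against a one-second accumulator to subtract health.
; Logic to add PuddleSize to the water table and destroy the puddle is present but disconnected.
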(event `DissolveWater`
  (bind _defaultsceneroot (`self.DefaultSceneRoot`))
  (bind (_returnvalue_x _returnvalue_y _returnvalue_z) (`KismetMathLibrary.BreakVector` (`SceneComponent.K2_GetComponentLocation` _defaultsceneroot)))
  ;[1 1 1] Dissolve Water into Water Table
  (`SceneComponent.K2_SetWorldLocation` _defaultsceneroot (`KismetMathLibrary.MakeVector` _returnvalue_x _returnvalue_y (- _returnvalue_z 1.0)) true false))

(event `self.ReceiveBeginPlay`
  ;[1 1 1] BeginPlay - Create and Assign Increase Water Level Despatch Message
  (`KismetSystemLibrary.K2_SetTimer` null "DissolveWater" 0.2 true))

(event `self.PaperSprite.OnComponentBeginOverlap`
  (params (OverlappedComponent :type "PrimitiveComponent Object Reference") (OtherActor :type "Actor Object Reference") (OtherComp :type "PrimitiveComponent Object Reference") (OtherBodyIndex :type Integer) (bFromSweep :type Boolean) (SweepResult :type "HitResult Structure (by ref)"))
  ;[1 1 1] Set Player is In Water when entering Water
  (cast `/Game/MyContent/Characters/BubbleCharacter/BubbleCharacter` OtherActor)
  (set `self.PlayerIsInWater` true))

(event `self.PaperSprite.OnComponentEndOverlap`
  (params (OverlappedComponent :type "PrimitiveComponent Object Reference") (OtherActor :type "Actor Object Reference") (OtherComp :type "PrimitiveComponent Object Reference") (OtherBodyIndex :type Integer))
  ;[1 1 1] Set Player Is In Water to false when exiting Water
  (cast `/Game/MyContent/Characters/BubbleCharacter/BubbleCharacter` OtherActor)
  (set `self.PlayerIsInWater` false))

(event `self.ReceiveTick`
  (params (DeltaSeconds :type "Float (single-precision)"))
  (bind _returnvalue (+ DeltaSeconds (`self.DeltaTime`)))
  ;[1 1 1] Event Tick - Every second reduce the health of the Player Overlapping Water
  (`TextRenderComponent.K2_SetText` (`self.TextRender`) (`KismetTextLibrary.Conv_DoubleToText` (`self.PuddleSize`) "HalfToEven"))
  (if (>= _returnvalue 1.0)
    (if (`self.PlayerIsInWater`)
      (bind _asbubble_character (cast `/Game/MyContent/Characters/BubbleCharacter/BubbleCharacter` (`GameplayStatics.GetPlayerCharacter` 0)))
      (`/Game/MyContent/Characters/BubbleCharacter/BubbleCharacter.UpdateHealth` _asbubble_character -25.0)
      (set `self.DeltaTime` 0.0))
    (else
      (set `self.DeltaTime` _returnvalue))))

(fn `UserConstructionScript`)