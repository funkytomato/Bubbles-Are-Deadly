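; Water table actor whose Paper sprite serves as a rising and falling body of water that hurts the player.
; Water level dispatcher events and absorbed Puddle_BP actors change the height by adjusting the sprite's Z scale, with absorbed puddles destroyed.
; Overlap events flag when BubbleCharacter is in the water, and a Tick timer applies health loss at roughly one-second intervals.
; Tick also polls all puddles, shortening the lifespan of overlapping ones.
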(event `DecreaseWaterHeight`
  (params (Scale :type "Float (double-precision)"))
  (bind (_returnvalue_x _returnvalue_y _returnvalue_z) (`KismetMathLibrary.BreakVector` (`SceneComponent.K2_GetComponentScale` (`self.PaperSprite`))))
  ;[1 1 1] Decrease the Water Level
  (`SceneComponent.SetWorldScale3D` (`self.PaperSprite`) (`KismetMathLibrary.MakeVector` _returnvalue_x _returnvalue_y (- _returnvalue_z Scale))))

(event `IncreaseWaterHeight`
  (params (Scale :type "Float (double-precision)"))
  (bind (_returnvalue_x _returnvalue_y _returnvalue_z) (`KismetMathLibrary.BreakVector` (`SceneComponent.K2_GetComponentScale` (`self.PaperSprite`))))
  ;[1 1 1] Increase the Water Level
  (`SceneComponent.SetWorldScale3D` (`self.PaperSprite`) (`KismetMathLibrary.MakeVector` _returnvalue_x _returnvalue_y (+ _returnvalue_z Scale))))

(event `self.ReceiveBeginPlay`
  ;[1 1 1] BeginPlay - Create and Assign Increase Water Level Despatch Message
  (add `self.IncreaseWaterLevel` (delegate `IncreaseWaterLevel_Event`))
  (add `self.DecreaseWaterLevel` (delegate `DecreaseWaterLevel_Event`)))

(event `DecreaseWaterLevel_Event` :!signature `self.DecreaseWaterLevel`
  (params (Amount :type "Float (double-precision)"))
  ;[1 1 1] BeginPlay - Create and Assign Increase Water Level Despatch Message
  (`self.DecreaseWaterHeight` Amount))

(event `IncreaseWaterLevel_Event` :!signature `self.IncreaseWaterLevel`
  (params (Amount :type "Float (double-precision)"))
  ;[1 1 1] BeginPlay - Create and Assign Increase Water Level Despatch Message
  (`self.IncreaseWaterHeight` Amount))

(event `self.PaperSprite.OnComponentBeginOverlap`
  (params (OverlappedComponent :type "PrimitiveComponent Object Reference") (OtherActor :type "Actor Object Reference") (OtherComp :type "PrimitiveComponent Object Reference") (OtherBodyIndex :type Integer) (bFromSweep :type Boolean) (SweepResult :type "HitResult Structure (by ref)"))
  ;[1 1 1] OnCollision - Reduce Player Health upon entering water, or Increase the Water Table Height
  (bind _asbubble_character (cast `/Game/MyContent/Characters/BubbleCharacter/BubbleCharacter` OtherActor)
    (:`then`
      (set `self.IsPlayerInWater` true))
    (:`CastFailed`
      ;[1 1 1] When Puddle Hits WaterTable increase height and destroy puddle
      (bind _aspuddle_bp (cast `/Game/MyContent/LevelItems/WaterLevel/Puddle_BP` OtherActor))
      (`/Engine/EditorBlueprintResources/StandardMacros.DoOnce` false :!label _label
        (:`Completed`
          (`self.IncreaseWaterHeight` (`/Game/MyContent/LevelItems/WaterLevel/Puddle_BP.PuddleSize` _aspuddle_bp))
          (`self.K2_DestroyActor` _aspuddle_bp)
          (goto _label :!via `Reset`))))))

(event `self.PaperSprite.OnComponentEndOverlap`
  (params (OverlappedComponent :type "PrimitiveComponent Object Reference") (OtherActor :type "Actor Object Reference") (OtherComp :type "PrimitiveComponent Object Reference") (OtherBodyIndex :type Integer))
  ;[1 1 1] Player has left Water
  (cast `/Game/MyContent/Characters/BubbleCharacter/BubbleCharacter` OtherActor)
  (set `self.IsPlayerInWater` false))

(event `self.ReceiveTick`
  (params (DeltaSeconds :type "Float (single-precision)"))
  (bind _returnvalue (+ DeltaSeconds (`self.DeltaTime`)))
  ;[1 1 1] Event Tick - Every second reduce the health of the Player Overlapping Water
  (if (>= _returnvalue 1.0)
    (if (`self.IsPlayerInWater`)
      (bind _asbubble_character (cast `/Game/MyContent/Characters/BubbleCharacter/BubbleCharacter` (`GameplayStatics.GetPlayerCharacter` 0)))
      (`/Game/MyContent/Characters/BubbleCharacter/BubbleCharacter.UpdateHealth` _asbubble_character -25.0)
      (set `self.DeltaTime` 0.0))
    (else
      (set `self.DeltaTime` _returnvalue)
      ;;[1 1 1] Comment
      (bind _outactors (`GameplayStatics.GetAllActorsOfClass` "/Game/MyContent/LevelItems/WaterLevel/Puddle_BP.Puddle_BP_C"))
      (for _array_element _outactors
        (if (`self.IsOverlappingActor` _array_element null)
          (`self.SetLifeSpan` _array_element 0.2)
          (`KismetSystemLibrary.PrintString` "Lifespan set"))))))

(fn `UserConstructionScript`)