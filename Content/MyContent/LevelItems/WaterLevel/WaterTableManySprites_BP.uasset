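; Water table hazard built from many Paper sprites that drains 25 player health at one-second intervals during overlap with its Box.
; Puddles hitting the Box raise the water by their size and are destroyed; bound level events also raise or lower it.
; Height changes step sprite Z scale without resizing the Box, though the decrease loop only writes to the first sprite.
; Tick also polls all puddles, setting short lifespans on overlapping ones.
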(event `DecreaseWaterHeight`
  (params (Scale :type "Float (double-precision)"))
  (`/Engine/EditorBlueprintResources/StandardMacros.DoOnce` false :!label _label
    (:`Completed`
      (for _array_element (`|MakeArray` (`self.PaperSprite`) (`self.PaperSprite1`) (`self.PaperSprite2`) (`self.PaperSprite3`) (`self.PaperSprite4`) (`self.PaperSprite5`) (`self.PaperSprite6`) (`self.PaperSprite7`) (`self.PaperSprite8`) (`self.PaperSprite9`) (`self.PaperSprite10`) (`self.PaperSprite11`) (`self.PaperSprite12`) (`self.PaperSprite13`) (`self.PaperSprite14`) (`self.PaperSprite15`) (`self.PaperSprite16`) (`self.PaperSprite17`) (`self.PaperSprite18`) (`self.PaperSprite19`) (`self.PaperSprite20`) (`self.PaperSprite21`) (`self.PaperSprite22`) (`self.PaperSprite23`) (`self.PaperSprite24`) (`self.PaperSprite25`) (`self.PaperSprite26`) (`self.PaperSprite27`) (`self.PaperSprite28`) (`self.PaperSprite29`) (`self.PaperSprite30`) (`self.PaperSprite31`) (`self.PaperSprite32`) (`self.PaperSprite33`) (`self.PaperSprite34`) (`self.PaperSprite35`) (`self.PaperSprite36`) (`self.PaperSprite37`) (`self.PaperSprite38`) (`self.PaperSprite39`) (`self.PaperSprite40`) (`self.PaperSprite41`) (`self.PaperSprite42`) (`self.PaperSprite43`) (`self.PaperSprite44`) (`self.PaperSprite45`) (`self.PaperSprite46`) (`self.PaperSprite47`) (`self.PaperSprite48`) (`self.PaperSprite49`) (`self.PaperSprite50`) (`self.PaperSprite51`) (`self.PaperSprite52`) (`self.PaperSprite53`) (`self.PaperSprite54`) (`self.PaperSprite55`) (`self.PaperSprite56`) (`self.PaperSprite57`) (`self.PaperSprite58`) (`self.PaperSprite59`) (`self.PaperSprite60`) (`self.PaperSprite61`) (`self.PaperSprite62`) (`self.PaperSprite63`) (`self.PaperSprite64`) (`self.PaperSprite65`) (`self.PaperSprite66`) (`self.PaperSprite67`) (`self.PaperSprite68`) (`self.PaperSprite69`) (`self.PaperSprite70`) (`self.PaperSprite71`) (`self.PaperSprite72`))
        (bind (_returnvalue_x _returnvalue_y _returnvalue_z) (`KismetMathLibrary.BreakVector` (`SceneComponent.K2_GetComponentScale` _array_element)))
        ;[1 1 1] Decrease the Water Level
        (`SceneComponent.SetWorldScale3D` (`self.PaperSprite`) (`KismetMathLibrary.MakeVector` _returnvalue_x _returnvalue_y (- _returnvalue_z Scale))))
      (goto _label :!via `Reset`))))

(event `IncreaseWaterHeight`
  (params (Scale :type "Float (double-precision)"))
  (`/Engine/EditorBlueprintResources/StandardMacros.DoOnce` false :!label _label_2
    (:`Completed`
      ;[1 1 1] Increase the Water Level
      (for _array_element (`|MakeArray` (`self.PaperSprite`) (`self.PaperSprite1`) (`self.PaperSprite2`) (`self.PaperSprite3`) (`self.PaperSprite4`) (`self.PaperSprite5`) (`self.PaperSprite6`) (`self.PaperSprite7`) (`self.PaperSprite8`) (`self.PaperSprite9`) (`self.PaperSprite10`) (`self.PaperSprite11`) (`self.PaperSprite12`) (`self.PaperSprite13`) (`self.PaperSprite14`) (`self.PaperSprite15`) (`self.PaperSprite16`) (`self.PaperSprite17`) (`self.PaperSprite18`) (`self.PaperSprite19`) (`self.PaperSprite20`) (`self.PaperSprite21`) (`self.PaperSprite22`) (`self.PaperSprite23`) (`self.PaperSprite24`) (`self.PaperSprite25`) (`self.PaperSprite26`) (`self.PaperSprite27`) (`self.PaperSprite28`) (`self.PaperSprite29`) (`self.PaperSprite30`) (`self.PaperSprite31`) (`self.PaperSprite32`) (`self.PaperSprite33`) (`self.PaperSprite34`) (`self.PaperSprite35`) (`self.PaperSprite36`) (`self.PaperSprite37`) (`self.PaperSprite38`) (`self.PaperSprite39`) (`self.PaperSprite40`) (`self.PaperSprite41`) (`self.PaperSprite42`) (`self.PaperSprite43`) (`self.PaperSprite44`) (`self.PaperSprite45`) (`self.PaperSprite46`) (`self.PaperSprite47`) (`self.PaperSprite48`) (`self.PaperSprite49`) (`self.PaperSprite50`) (`self.PaperSprite51`) (`self.PaperSprite52`) (`self.PaperSprite53`) (`self.PaperSprite54`) (`self.PaperSprite55`) (`self.PaperSprite56`) (`self.PaperSprite57`) (`self.PaperSprite58`) (`self.PaperSprite59`) (`self.PaperSprite60`) (`self.PaperSprite61`) (`self.PaperSprite62`) (`self.PaperSprite63`) (`self.PaperSprite64`) (`self.PaperSprite65`) (`self.PaperSprite66`) (`self.PaperSprite67`) (`self.PaperSprite68`) (`self.PaperSprite69`) (`self.PaperSprite70`) (`self.PaperSprite71`) (`self.PaperSprite72`))
        (bind (_returnvalue_x _returnvalue_y _returnvalue_z) (`KismetMathLibrary.BreakVector` (`SceneComponent.K2_GetComponentScale` _array_element)))
        (`SceneComponent.SetWorldScale3D` _array_element (`KismetMathLibrary.MakeVector` _returnvalue_x _returnvalue_y (+ _returnvalue_z Scale))))
      (goto _label_2 :!via `Reset`))))

(event `self.ReceiveBeginPlay`
  ;[1 1 1] BeginPlay - Create and Assign Increase Water Level Despatch Message
  (add `self.IncreaseWaterLevel` (delegate `IncreaseWaterLevel_Event`))
  (add `self.DecreaseWaterLevel` (delegate `DecreaseWaterLevel_Event`)))

(event `DecreaseWaterLevel_Event` :!signature `self.DecreaseWaterLevel`
  (params (Amount :type "Float (double-precision)"))
  ;[1 1 1] BeginPlay - Create and Assign Increase Water Level Despatch Message
  (`self.DecreaseWaterHeight` Amount))

(event `IncreaseWaterLevel_Event` :!signature `self.IncreaseWaterLevel`
  (params (Amount :type "Float (double-precision)"))
  ;[1 1 1] BeginPlay - Create and Assign Increase Water Level Despatch Message
  (`self.IncreaseWaterHeight` Amount))

(event `self.Box.OnComponentEndOverlap`
  (params (OverlappedComponent :type "PrimitiveComponent Object Reference") (OtherActor :type "Actor Object Reference") (OtherComp :type "PrimitiveComponent Object Reference") (OtherBodyIndex :type Integer))
  ;[1 1 1] Player has left Water
  (cast `/Game/MyContent/Characters/BubbleCharacter/BubbleCharacter` OtherActor)
  (set `self.IsPlayerInWater` false))

(event `self.ReceiveTick`
  (params (DeltaSeconds :type "Float (single-precision)"))
  (bind _returnvalue (+ DeltaSeconds (`self.DeltaTime`)))
  ;[1 1 1] Event Tick - Every second reduce the health of the Player Overlapping Water
  (if (>= _returnvalue 1.0)
    (if (`self.IsPlayerInWater`)
      (bind _asbubble_character (cast `/Game/MyContent/Characters/BubbleCharacter/BubbleCharacter` (`GameplayStatics.GetPlayerCharacter` 0)))
      (`/Game/MyContent/Characters/BubbleCharacter/BubbleCharacter.UpdateHealth` _asbubble_character -25.0)
      (set `self.DeltaTime` 0.0))
    (else
      (set `self.DeltaTime` _returnvalue)
      ;;[1 1 1] Comment
      (bind _outactors (`GameplayStatics.GetAllActorsOfClass` "/Game/MyContent/LevelItems/Puddles/Puddle_BP.Puddle_BP_C"))
      (for _array_element _outactors
        (if (`self.IsOverlappingActor` _array_element null)
          (`self.SetLifeSpan` _array_element 0.2)
          (`KismetSystemLibrary.PrintString` "Lifespan set"))))))

(event `self.Box.OnComponentBeginOverlap`
  (params (OverlappedComponent :type "PrimitiveComponent Object Reference") (OtherActor :type "Actor Object Reference") (OtherComp :type "PrimitiveComponent Object Reference") (OtherBodyIndex :type Integer) (bFromSweep :type Boolean) (SweepResult :type "HitResult Structure (by ref)"))
  ;[1 1 1] OnCollision - Reduce Player Health upon entering water, or Increase the Water Table Height
  (cast `/Game/MyContent/Characters/BubbleCharacter/BubbleCharacter` OtherActor
    (:`then`
      (set `self.IsPlayerInWater` true))
    (:`CastFailed`
      ;[1 1 1] When Puddle Hits WaterTable increase height and destroy puddle
      (bind _aspuddle_bp (cast `/Game/MyContent/LevelItems/Puddles/Puddle_BP` OtherActor))
      (`/Engine/EditorBlueprintResources/StandardMacros.DoOnce` false :!label _label_3
        (:`Completed`
          (`self.IncreaseWaterHeight` (`/Game/MyContent/LevelItems/Puddles/Puddle_BP.PuddleSize` _aspuddle_bp))
          (`self.K2_DestroyActor` _aspuddle_bp)
          (goto _label_3 :!via `Reset`))))))

(fn `UserConstructionScript`)