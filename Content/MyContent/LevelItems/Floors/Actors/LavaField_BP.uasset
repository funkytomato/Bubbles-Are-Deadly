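; LavaField_BP is a lava floor hazard that reacts to bubbles overlapping its Collision component.
; A BubbleCharacter that enters is sent a health update of -25 through UpdateHealthMsg, along with a debug "Hello" print.
; A PhysicsBubble_BP that enters instead turns the field's three Paper2D sprites black, with no reset and no change to the damage behavior.
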(event `self.Collision.OnComponentBeginOverlap`
  (params (OverlappedComponent :type "PrimitiveComponent Object Reference") (OtherActor :type "Actor Object Reference") (OtherComp :type "PrimitiveComponent Object Reference") (OtherBodyIndex :type Integer) (bFromSweep :type Boolean) (SweepResult :type "HitResult Structure (by ref)"))
  (bind _asbubble_character (cast `/Game/MyContent/Characters/BubbleCharacter/BubbleCharacter` OtherActor)
    (:`then`
      (`/Game/MyContent/Characters/BubbleCharacter/BubbleCharacter.UpdateHealthMsg` _asbubble_character -25.0)
      (`KismetSystemLibrary.PrintString` "Hello"))
    (:`CastFailed`
      (cast `/Game/MyContent/LevelItems/Bubbles/PhysicsBubble_BP` OtherActor)
      (`|ExecutionSequence`
        (:`then_0`
          (`PaperSpriteComponent.SetSpriteColor` :`self` (`self.PaperSprite2`)))
        (:`then_1`
          (`PaperSpriteComponent.SetSpriteColor` :`self` (`self.PaperSprite3`)))
        (:`then_2`
          (`PaperSpriteComponent.SetSpriteColor` :`self` (`self.PaperSprite1`)))))))

(fn `UserConstructionScript`)