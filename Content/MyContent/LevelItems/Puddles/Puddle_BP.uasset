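; Puddle level item that drains the player's health while a BubbleCharacter stands in it.
; Collision begin and end overlap events toggle a PlayerIsInWater flag.
; A looping quarter-second timer started on BeginPlay, used in place of Tick, checks that flag and applies a fixed health penalty to player character 0 through CallUpdateHealth.
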(event `self.ReceiveBeginPlay`
  ;[1 1 1] BeginPlay - Set Timer for PlayerInWaterCheck
  (`KismetSystemLibrary.K2_SetTimer` null "CheckPlayerInWater" 0.25 true))

(event `self.Collision.OnComponentBeginOverlap`
  (params (OverlappedComponent :type "PrimitiveComponent Object Reference") (OtherActor :type "Actor Object Reference") (OtherComp :type "PrimitiveComponent Object Reference") (OtherBodyIndex :type Integer) (bFromSweep :type Boolean) (SweepResult :type "HitResult Structure (by ref)"))
  ;[1 1 1] Set Player is In Water when entering Water
  (cast `/Game/MyContent/Characters/BubbleCharacter/BubbleCharacter` OtherActor)
  (set `self.PlayerIsInWater` true))

(event `self.Collision.OnComponentEndOverlap`
  (params (OverlappedComponent :type "PrimitiveComponent Object Reference") (OtherActor :type "Actor Object Reference") (OtherComp :type "PrimitiveComponent Object Reference") (OtherBodyIndex :type Integer))
  ;[1 1 1] Set Player Is In Water to false when exiting Water
  (cast `/Game/MyContent/Characters/BubbleCharacter/BubbleCharacter` OtherActor)
  (set `self.PlayerIsInWater` false))

(event `CheckPlayerInWater`
  ;[1 1 1] Event Tick - Every second reduce the health of the Player Overlapping Water
  (if (`self.PlayerIsInWater`)
    (bind _asbubble_character (cast `/Game/MyContent/Characters/BubbleCharacter/BubbleCharacter` (`GameplayStatics.GetPlayerCharacter` 0)))
    (`/Game/MyContent/Characters/BubbleCharacter/BubbleCharacter.UpdateHealth` _asbubble_character -5.0)))

(fn `UserConstructionScript`)