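; Freeze pickup actor that freezes the physics bubble that owns it.
; On BeginPlay it casts its owner to PhysicsBubble_BP, calls FreezeBubble on it, then destroys itself after a brief delay.
; A disconnected branch holds an area version that would freeze every bubble overlapping FreezeInfluenceArea, with debug prints, but it never runs.
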(event `self.ReceiveBeginPlay`
  (bind _asphysics_bubble_bp (cast `/Game/MyContent/LevelItems/Bubbles/PhysicsBubble_BP` (`self.GetOwner`)))
  (`/Game/MyContent/LevelItems/Bubbles/PhysicsBubble_BP.FreezeBubble` _asphysics_bubble_bp)
  (`KismetSystemLibrary.Delay` 0.1)
  (`self.K2_DestroyActor`))

(fn `UserConstructionScript`)