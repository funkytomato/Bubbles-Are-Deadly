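; HealthPickup_BP is a health pickup that adds a fixed amount to a BubbleCharacter's Health, with no clamp here, when it overlaps the Collision component, then destroys itself.
; Its PaperSprite hit event tests for four ground Blueprint types through chained casts.
; A hit on any of them leads to a shared delayed destroy, so landed pickups expire after a few seconds.
; A SetLifeSpan node is left unconnected.
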(event `self.ReceiveBeginPlay`)

(event `self.Collision.OnComponentBeginOverlap`
  (params (OverlappedComponent :type "PrimitiveComponent Object Reference") (OtherActor :type "Actor Object Reference") (OtherComp :type "PrimitiveComponent Object Reference") (OtherBodyIndex :type Integer) (bFromSweep :type Boolean) (SweepResult :type "HitResult Structure (by ref)"))
  (bind _asbubble_character (cast `/Game/MyContent/Characters/BubbleCharacter/BubbleCharacter` OtherActor))
  (set `/Game/MyContent/Characters/BubbleCharacter/BubbleCharacter.Health` (+ (`/Game/MyContent/Characters/BubbleCharacter/BubbleCharacter.Health` _asbubble_character) 10.0) _asbubble_character)
  (`self.K2_DestroyActor`))

(event `self.PaperSprite.OnComponentHit`
  (params (HitComponent :type "PrimitiveComponent Object Reference") (OtherActor :type "Actor Object Reference") (OtherComp :type "PrimitiveComponent Object Reference") (NormalImpulse :type "Vector Structure") (Hit :type "HitResult Structure (by ref)"))
  (cast `/Game/MyContent/LevelItems/Floors/Actors/BubbleGround_BP` OtherActor
    (:`then`
      _)
    (:`CastFailed`
      (cast `/Game/MyContent/LevelItems/Floors/Actors/BaseGroundContinous_BP` OtherActor
        (:`then`
          _)
        (:`CastFailed`
          (cast `/Game/MyContent/LevelItems/Floors/Actors/BaseGroundLeft_BP` OtherActor
            (:`then`
              _)
            (:`CastFailed`
              (cast `/Game/MyContent/LevelItems/Floors/Actors/BaseGroundRight_BP` OtherActor)))))))
  (`KismetSystemLibrary.Delay` 5.0)
  (`self.K2_DestroyActor`))

(fn `UserConstructionScript`)