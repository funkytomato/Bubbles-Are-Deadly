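; WaterEvaporatorPickup_BP is a single-use pickup that evaporates water when it overlaps a WaterTableManySprites_BP actor.
; On overlap it lowers that water table's level by a configurable amount.
; It then strengthens the wind of the CloudRandomDestination_BP actors cached at BeginPlay, adding to their radial force and reapplying it.
; The pickup destroys itself afterwards.
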(event `self.ReceiveBeginPlay`
  ;[1 1 1] Create an array of Clouds in Game
  (bind _outactors (`GameplayStatics.GetAllActorsOfClass` "/Game/MyContent/LevelItems/WindForce/CloudRandomDestination_BP.CloudRandomDestination_BP_C")))

(event `self.Collision.OnComponentBeginOverlap`
  (params (OverlappedComponent :type "PrimitiveComponent Object Reference") (OtherActor :type "Actor Object Reference") (OtherComp :type "PrimitiveComponent Object Reference") (OtherBodyIndex :type Integer) (bFromSweep :type Boolean) (SweepResult :type "HitResult Structure (by ref)"))
  ;[1 1 1] Reduce the Water level because of evaporation!
  (bind _aswater_table_many_sprites_bp (cast `/Game/MyContent/LevelItems/WaterLevel/WaterTableManySprites_BP` OtherActor))
  (`/Game/MyContent/LevelItems/WaterLevel/WaterTableManySprites_BP.DecreaseWaterLevel` _aswater_table_many_sprites_bp (`self.WaterLevelToDecrease`))
  ;[1 1 1] Evaporation causes clouds to be be windier
  (for _array_element (stale `self.ReceiveBeginPlay` _outactors)
    (bind _ascloud_random_destination_bp (cast `/Game/MyContent/LevelItems/WindForce/CloudRandomDestination_BP` _array_element))
    (set `/Game/MyContent/LevelItems/WindForce/CloudRandomDestination_BP.ForceStrength` (+ (`RadialForceComponent.ForceStrength` (`/Game/MyContent/LevelItems/WindForce/CloudRandomDestination_BP.RadialForce` _ascloud_random_destination_bp)) (`self.WindForceToApply`)) _ascloud_random_destination_bp)
    (`/Game/MyContent/LevelItems/WindForce/CloudRandomDestination_BP.SetForces` _ascloud_random_destination_bp))
  (`self.K2_DestroyActor`))

(fn `UserConstructionScript`)