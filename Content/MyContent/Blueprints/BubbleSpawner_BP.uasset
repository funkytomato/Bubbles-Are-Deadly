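; Bubble spawner that manages the bubble population of a level, from timed spawning to completion.
; A looping timer spawns bubbles at random points under alive and created count limits, with size setting scale, mass and point value.
; Popping above a height threshold splits bubbles into mostly smaller ones, merging creates larger ones, and a separate event spawns puddles.
; Tick shows the Game Instance's level-complete menu once the quota is created and none remain alive.
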(event `self.ReceiveBeginPlay`
  ;[1 1 1] BeginPlay - Set the Game Instance and Timer for Bubble Spawner
  (bind _asbubble_game_instance (cast `/Game/MyContent/Blueprints/BubbleGameInstance` (`GameplayStatics.GetGameInstance`)))
  (set `self.GameInstance` _asbubble_game_instance)
  (`self.CreateBubbles`)
  (`KismetSystemLibrary.K2_SetTimerDelegate` (delegate `Create Bubble`) (`self.Frequency`) true))

(event `Create Bubble`
  ;[1 1 1] BeginPlay - Set the Game Instance and Timer for Bubble Spawner
  (`self.CreateBubbles`))

(event `IncrementBubbleAliveCount`
  ;[1 1 1] Increment Total Bubble Alive Count
  (set `self.TotalBubblesAlive` (`KismetMathLibrary.Clamp` (+ (`self.TotalBubblesAlive`) 1) 0 (`self.MaxBubblesInLevel`))))

(event `SpawnBubbles`
  (params (Size :type "/Game/MyContent/Blueprints/BubbleSize Enum" :default "NewEnumerator0") (SpawnLocation :type "Vector Structure") (BubblesToCreate :type Integer))
  (bind _bubblecountloop (`self.BubbleCountLoop`))
  ;[1 1 1] Spawn Bubbles
  ;;[1 1 1] Bubbles shall not exceed maximum bubble alive count, we don't want too may bubbles in play
  (if (<= (`self.TotalBubblesAlive`) (`self.MaximumAliveBubbles`))
    ;;[1 1 1] Bubbles created shall not exceed maximum bubble count
    (if (<= (`self.BubblesCreatedCount`) (`self.MaxBubblesInLevel`))
      (if (<= _bubblecountloop (`self.MaxBubblesInLevel`))
        (while (< _bubblecountloop BubblesToCreate)
          (if true
            (`self.SpawnBubble` SpawnLocation Size)
            (set `self.BubbleCountLoop` (+ (`self.BubbleCountLoop`) 1))
            (`KismetSystemLibrary.Delay` 0.3)))
        (set `self.BubbleCountLoop` 0)))
    (else
      (`KismetSystemLibrary.PrintString` "Too many bubbles"))))

(event `IncrementBubblesCreatedCount`
  ;[1 1 1] Increment Bubbles Created Count
  (set `self.BubblesCreatedCount` (+ (`self.BubblesCreatedCount`) 1)))

(event `PopBubble`
  (params (size :type "/Game/MyContent/Blueprints/BubbleSize Enum" :default "NewEnumerator0") (SpawnLocation :type "Vector Structure"))
  ;[1 1 1] Pop a Bubble (Main Call)
  (bind _output_get (set `self.SpawnLocation` SpawnLocation))
  (if (> (.z _output_get) (`self.LowestBubblePopPoint`))
    (switch `/Game/MyContent/Blueprints/BubbleSize` size
      (:`NewEnumerator5`
        (`self.SpawnBubbles` "NewEnumerator0" SpawnLocation (`KismetMathLibrary.RandomIntegerInRange` 1 2))
        (`self.SpawnBubbles` "NewEnumerator1" SpawnLocation (`KismetMathLibrary.RandomIntegerInRange` 1 2)))
      (:`NewEnumerator0`
        (`self.SpawnBubbles` "NewEnumerator1" SpawnLocation (`KismetMathLibrary.RandomIntegerInRange` 1 2))
        (`self.SpawnBubbles` "NewEnumerator2" SpawnLocation (`KismetMathLibrary.RandomIntegerInRange` 1 2)))
      (:`NewEnumerator1`
        (`self.SpawnBubbles` "NewEnumerator2" SpawnLocation (`KismetMathLibrary.RandomIntegerInRange` 1 2))
        (`self.SpawnBubbles` "NewEnumerator3" SpawnLocation (`KismetMathLibrary.RandomIntegerInRange` 1 2)))
      (:`NewEnumerator2`
        (`self.SpawnBubbles` "NewEnumerator3" SpawnLocation (`KismetMathLibrary.RandomIntegerInRange` 1 2))
        (`self.SpawnBubbles` "NewEnumerator2" SpawnLocation (`KismetMathLibrary.RandomIntegerInRange` 1 2)))
      (:`NewEnumerator3`
        (`self.SpawnBubbles` "NewEnumerator4" SpawnLocation (`KismetMathLibrary.RandomIntegerInRange` 1 3))))))

(event `DecrementBubbleAliveCount`
  ;[1 1 1] Decrement Total Bubbles Alive Count
  (set `self.TotalBubblesAlive` (`KismetMathLibrary.Clamp` (- (`self.TotalBubblesAlive`) 1) 0 (`self.MaxBubblesInLevel`))))

(event `SpawnBubble`
  (params (Location :type "Vector Structure") (Size :type "/Game/MyContent/Blueprints/BubbleSize Enum" :default "NewEnumerator0"))
  ;[1 1 1] Spawn a Single Bubble
  (set `self.SpawnProximity` (* (select `/Game/MyContent/Blueprints/BubbleSize` Size :`NewEnumerator5` (`self.EnormousSize`) :`NewEnumerator0` (`self.HugeSize`) :`NewEnumerator1` (`self.LargeSize`) :`NewEnumerator2` (`self.MediumSize`) :`NewEnumerator3` (`self.SmallSize`) :`NewEnumerator4` (`self.TinySize`)) 100.0))
  (bind _returnvalue (`|SpawnActorFromClass` "/Game/MyContent/LevelItems/Bubbles/PhysicsBubble_BP.PhysicsBubble_BP_C" (`KismetMathLibrary.MakeTransform` (`KismetMathLibrary.MakeVector` (`KismetMathLibrary.RandomFloatInRange` (- Location_X (`self.SpawnProximity`)) (+ Location_X (`self.SpawnProximity`))) 0.0 (`KismetMathLibrary.RandomFloatInRange` (- Location_Z (`self.SpawnProximity`)) (+ Location_Z (`self.SpawnProximity`)))) (struct) (`KismetMathLibrary.Conv_DoubleToVector` (select `/Game/MyContent/Blueprints/BubbleSize` Size :`NewEnumerator5` (`self.EnormousSize`) :`NewEnumerator0` (`self.HugeSize`) :`NewEnumerator1` (`self.LargeSize`) :`NewEnumerator2` (`self.MediumSize`) :`NewEnumerator3` (`self.SmallSize`) :`NewEnumerator4` (`self.TinySize`)))) "AdjustIfPossibleButDontSpawnIfColliding" "OverrideRootScale" null null))
  ;;[1 1 1] Check Bubble is not pending death
  (if (`KismetSystemLibrary.IsValid` _returnvalue)
    (set `/Game/MyContent/LevelItems/Bubbles/PhysicsBubble_BP.BubbleSize` Size _returnvalue)
    (`PrimitiveComponent.SetMassOverrideInKg` (`/Game/MyContent/LevelItems/Bubbles/PhysicsBubble_BP.BubbleCollision` _returnvalue) "None" (select `/Game/MyContent/Blueprints/BubbleSize` Size :`NewEnumerator5` (`self.EnormousSize`) :`NewEnumerator0` (`self.HugeSize`) :`NewEnumerator1` (`self.LargeSize`) :`NewEnumerator2` (`self.MediumSize`) :`NewEnumerator3` (`self.SmallSize`) :`NewEnumerator4` (`self.TinySize`)) true)
    (`self.IncrementBubbleAliveCount`)
    (`self.IncrementBubblesCreatedCount`)
    (set `/Game/MyContent/LevelItems/Bubbles/PhysicsBubble_BP.PointValue` (select `/Game/MyContent/Blueprints/BubbleSize` Size :`NewEnumerator5` (`self.EnormousPointValue`) :`NewEnumerator0` (`self.HugePointValue`) :`NewEnumerator1` (`self.LargePointValue`) :`NewEnumerator2` (`self.MediumPointValue`) :`NewEnumerator3` (`self.SmallPointValue`) :`NewEnumerator4` (`self.TinyPointValue`)) _returnvalue)))

(event `SpawnPuddle`
  (params (SpawnLocation :type "Vector Structure") (PuddleSize :type "/Game/MyContent/Blueprints/BubbleSize Enum" :default "NewEnumerator0"))
  ;[1 1 1] Spawn Puddle at Location and Set its Size respective to the Bubble Size
  (bind _returnvalue (`|SpawnActorFromClass` "/Game/MyContent/LevelItems/Puddles/Puddle_BP.Puddle_BP_C" (`KismetMathLibrary.MakeTransform` (`KismetMathLibrary.MakeVector` SpawnLocation_X 0.0 -9.0)) "AdjustIfPossibleButDontSpawnIfColliding" "OverrideRootScale" null null))
  (if (`KismetSystemLibrary.IsValid` _returnvalue)
    (set `/Game/MyContent/LevelItems/Puddles/Puddle_BP.PuddleSize` (select `/Game/MyContent/Blueprints/BubbleSize` PuddleSize :`NewEnumerator5` 2.0 :`NewEnumerator0` (`self.HugeSize`) :`NewEnumerator1` (`self.LargeSize`) :`NewEnumerator2` (`self.MediumSize`) :`NewEnumerator3` (`self.SmallSize`) :`NewEnumerator4` (`self.TinySize`)) _returnvalue)))

(event `ResetBubbleCount`
  ;[1 1 1] Reset Bubble Count
  (set `self.BubbleCountLoop` 0)
  (set `self.TotalBubblesAlive` 0))

(event `MergeBubbles`
  (params (BubbleA :type "/Game/MyContent/LevelItems/Bubbles/PhysicsBubble_BP Object Reference") (BubbleB :type "/Game/MyContent/LevelItems/Bubbles/PhysicsBubble_BP Object Reference") (ContactLocation :type "Vector Structure"))
  (bind _bubblesize (`/Game/MyContent/LevelItems/Bubbles/PhysicsBubble_BP.BubbleSize` BubbleA))
  (bind _bubblesize_2 (`/Game/MyContent/LevelItems/Bubbles/PhysicsBubble_BP.BubbleSize` BubbleB))
  ;[1 1 1] Merge two bubbles together
  (if (or (`|EnumEquality` _bubblesize "NewEnumerator0") (`|EnumEquality` _bubblesize_2 "NewEnumerator0"))
    (`self.SpawnBubble` ContactLocation "NewEnumerator5")
    (`self.SetLifeSpan` BubbleA 0.1)
    (`self.SetLifeSpan` BubbleB 0.1)
    (elif (or (`|EnumEquality` _bubblesize "NewEnumerator1") (`|EnumEquality` _bubblesize_2 "NewEnumerator1"))
      (`self.SpawnBubble` ContactLocation)
      (`self.SetLifeSpan` BubbleA 0.1)
      (`self.SetLifeSpan` BubbleB 0.1)
      (elif (or (`|EnumEquality` _bubblesize "NewEnumerator2") (`|EnumEquality` _bubblesize_2 "NewEnumerator2"))
        (`self.SpawnBubble` ContactLocation "NewEnumerator1")
        (`self.SetLifeSpan` BubbleA 0.1)
        (`self.SetLifeSpan` BubbleB 0.1)
        (elif (or (`|EnumEquality` _bubblesize "NewEnumerator3") (`|EnumEquality` _bubblesize_2 "NewEnumerator3"))
          (`self.SpawnBubble` ContactLocation "NewEnumerator2")
          (`self.SetLifeSpan` BubbleA 0.1)
          (`self.SetLifeSpan` BubbleB 0.1)
          (elif (or (`|EnumEquality` _bubblesize "NewEnumerator4") (`|EnumEquality` _bubblesize_2 "NewEnumerator4"))
            (`self.SpawnBubble` ContactLocation "NewEnumerator3")
            (`self.SetLifeSpan` BubbleA 0.1)
            (`self.SetLifeSpan` BubbleB 0.1)))))))

(event `self.ReceiveTick`
  (params (DeltaSeconds :type "Float (single-precision)"))
  ;[1 1 1] Check all Bubbles have been created and destroyed, Show Level Complete Menu
  (if (>= (`self.BubblesCreatedCount`) (`self.MaxBubblesInLevel`))
    (if (== (`self.TotalBubblesAlive`) 0)
      (`/Game/MyContent/Blueprints/BubbleGameInstance.ShowLevelCompleteMenu` (`self.GameInstance`)))))

(fn `CreateBubbles`
  (bind _result (`/Engine/EditorBlueprintResources/StandardMacros.DecrementInt` (`self.BubblesToCreateEachTick`))
    (:`  `
      (while (<= (`self.TickBubbleCount`) _result)
        (`self.SpawnBubbles` "NewEnumerator0" (`KismetMathLibrary.MakeVector` (`KismetMathLibrary.RandomFloatInRange` (`self.LeftMostSpawnPoint`) (`self.RightMostSpawnPoint`)) 0.0 (`KismetMathLibrary.RandomFloatInRange` (`self.LowestSpawnPoint`) (`self.HighestSpawnPoint`))) 1)
        (set `self.TickBubbleCount` (+ (`self.TickBubbleCount`) 1)))
      (set `self.TickBubbleCount` 0))))

(fn `RetrieveBubbleSize`
  (params (BubbleSize :type "/Game/MyContent/Blueprints/BubbleSize Enum" :default "NewEnumerator5"))
  (returns (Size :type "Float (double-precision)"))
  (return (select `/Game/MyContent/Blueprints/BubbleSize` BubbleSize :`NewEnumerator0` (`self.HugeSize`) :`NewEnumerator1` (`self.LargeSize`) :`NewEnumerator2` (`self.MediumSize`) :`NewEnumerator3` (`self.SmallSize`) :`NewEnumerator4` (`self.TinySize`))))

(fn `UserConstructionScript`)